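; BP_Puerta is a door actor that opens either with the E key or remotely, as chosen by AbrirRemoto.
; In key mode, E toggles it while the player overlaps TriggerVolume; Open, Close and OpenClose events allow external control.
; The OpenDoor timeline either swings or scales the Hinge, per RotarEscalar, reversing to close and flipping IsOpen when finished.
; The construction script applies frame and leaf materials, labels the mode and shows IDs for remote doors.
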(event `Open`
  (if (not (`self.IsOpen`))
    (bind (_direction _x) (`Timeline|OpenDoor` :!via `PlayFromStart` :!label _label)
      (:`Update`
        (if (`self.Rotar/Escalar`)
          (`SceneComponent.K2_SetRelativeRotation` (`self.Hinge`) (`KismetMathLibrary.MakeRotator` 0.0 0.0 (* _x 95.0)) false false)
          (else
            (`SceneComponent.SetRelativeScale3D` (`self.Hinge`) (`KismetMathLibrary.VLerp` (0.2 1.0 1.0) (0.0 1.0 1.0) _x)))))
      (:`Finished`
        (set `self.IsOpen` (not (`self.IsOpen`)))))))

(event `self.TriggerVolume.OnComponentBeginOverlap`
  (params (OverlappedComponent :type "PrimitiveComponent Object Reference") (OtherActor :type "Actor Object Reference") (OtherComp :type "PrimitiveComponent Object Reference") (OtherBodyIndex :type Integer) (bFromSweep :type Boolean) (SweepResult :type "HitResult Structure (by ref)"))
  (if (== OtherActor (`GameplayStatics.GetPlayerCharacter` 0))
    (set `self.IsIn` true)))

(event `OpenClose`
  (params (a :type Boolean))
  (set `self.IsOpen` a)
  (if (`self.IsOpen`) :!label _label_2
    (`|ExecutionSequence` :!label _label_3
      (:`then_0`
        (goto _label :!via `Stop`))
      (:`then_1`
        (goto _label :!via `Reverse`)))
    (else
      (goto _label :!via `PlayFromStart`))))

(event `Key|E` :consume false
  (params (Key :type "Key Structure"))
  (:`Pressed`
    (if (not (`self.AbrirRemoto`))
      (if (`self.IsIn`)
        (goto _label_2)))))

(event `self.TriggerVolume.OnComponentEndOverlap`
  (params (OverlappedComponent :type "PrimitiveComponent Object Reference") (OtherActor :type "Actor Object Reference") (OtherComp :type "PrimitiveComponent Object Reference") (OtherBodyIndex :type Integer))
  (if (== OtherActor (`GameplayStatics.GetPlayerCharacter` 0))
    (set `self.IsIn` false)))

(event `Close`
  (if (`self.IsOpen`)
    (goto _label_3)))

(event `self.ReceiveBeginPlay`
  (if (not (`self.AbrirRemoto`))
    (`self.EnableInput` (`GameplayStatics.GetPlayerController` 0))))

(fn `UserConstructionScript`
  (bind _modo_de_abir2 (`self.Modo de abir2`))
  (bind _id2 (`self.ID2`))
  (`PrimitiveComponent.SetMaterial` (`self.Size1`) 0 (`self.MaterialMarco`))
  (`PrimitiveComponent.SetMaterial` (`self.Size2`) 0 (`self.MaterialMarco`))
  (`PrimitiveComponent.SetMaterial` (`self.Top`) 0 (`self.MaterialMarco`))
  (`PrimitiveComponent.SetMaterial` (`self.Leaf`) 0 (`self.MaterialPuerta`))
  (`TextRenderComponent.K2_SetText` (`self.ID1`) (`KismetTextLibrary.Conv_IntToText` (`self.ID`)))
  (`TextRenderComponent.K2_SetText` (`self.ID2`) (`KismetTextLibrary.Conv_IntToText` (`self.ID`)))
  (if (`self.AbrirRemoto`)
    (`TextRenderComponent.K2_SetText` _modo_de_abir2 "Con ID")
    (`SceneComponent.SetVisibility` _id2 true false)
    (`SceneComponent.SetVisibility` (`self.ID1`) true false)
    (else
      (`TextRenderComponent.K2_SetText` _modo_de_abir2 "Pulsar E")
      (`SceneComponent.SetVisibility` _id2 false false)
      (`SceneComponent.SetVisibility` (`self.ID1`) false false))))